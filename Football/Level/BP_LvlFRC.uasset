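; Level controller for a football formation editor, where formations are listed, added, removed and edited under a spawned top-down camera.
; BeginPlay loads or creates the SO_FormationData save object, spawns a FormationFactory and creates list and edit widgets that call back into this Blueprint.
; Editing an item swaps widgets and enables mouse input: a cursor trace selects a pawn or moves the selected one.
; Saving writes the factory's pawn positions into the current formation.
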(event `self.ReceiveBeginPlay`
  ;[1 1 1] Init
  (`self.SetUpCamera`)
  (`self.SetUpFormationData`)
  (`self.SetUpFormationFactory`)
  (`self.SetUpWidget`))

(event `/Game/Football/Interface/InterFaceListView.OnClickX`
  (params (Item :type "Object Object Reference"))
  (bind _formationdata (`self.FormationData`))
  ;[1 1 1] Remove Item
  (bind _id (`/Game/Football/Widget/Wg_List.GetItemId` (`self.WidgetList`) Item))
  (`/Game/Football/SaveObject/SO_FormationData.RemoveFormationAt` (`self.FormationData`) _id)
  (`/Game/Football/SaveObject/SO_Texts.CheckEmpty` _formationdata "NewEnumerator2")
  (`/Game/Football/Widget/Wg_List.LoadList` (`self.WidgetList`) (`/Game/Football/SaveObject/SO_Texts.Texts` _formationdata)))

(event `/Game/Football/Interface/InterFaceListView.OnClickAdd`
  (params (WidgetType :type "/Game/Football/Enum/WidgetType Enum" :default "NewEnumerator2"))
  ;[1 1 1] Add item
  (bind _text (`/Game/Football/SaveObject/SO_Texts.AddDefaultText` (`self.FormationData`) WidgetType))
  (`/Game/Football/Widget/Wg_List.AddName` (`self.WidgetList`) _text))

(event `InputAction|LeftMouseButtonDown`
  (params (Key :type "Key Structure"))
  (bind (_bblockinghit _binitialoverlap _time _distance _location _impactpoint _normal _impactnormal _physmat _hitactor) (`GameplayStatics.BreakHitResult` (`PlayerController.GetHitResultUnderCursorByChannel` (`GameplayStatics.GetPlayerController` 0) "TraceTypeQuery1" true)))
  ;[1 1 1] Left mouse event
  (:`Pressed`
    (bind _asplayer_pawn (cast `/Game/Football/GameObject/PlayerPawn` _hitactor)
      (:`then`
        (`/Game/Football/Factory/FormationFactory.SetSelectPawn` (`self.FormationFactory`) _asplayer_pawn))
      (:`CastFailed`
        (`self.K2_SetActorLocation` (`/Game/Football/Factory/FormationFactory.CurrentSelectPawn` (`self.FormationFactory`)) _location false false)))))

(event `/Game/Football/Interface/InterFaceListView.OnClickItem`
  (params (Item :type "Object Object Reference"))
  ;[1 1 1] Edit Item
  (bind _astext_object_wrapper (cast `/Game/Football/SaveObject/Text_ObjectWrapper` Item))
  (`/Game/Football/Widget/WG_ListEdit.SetSaveBtnTxt` (`self.WidgetListEdit`) (`/Game/Football/SaveObject/Text_ObjectWrapper.Name` _astext_object_wrapper))
  (bind _id (`/Game/Football/Widget/Wg_List.GetItemId` (`self.WidgetList`) Item))
  (set `self.CurrentId` _id)
  (`/Game/Football/Factory/FormationFactory.SetDefaultSelectPawn` (`self.FormationFactory`))
  (`self.EnableInput` (`GameplayStatics.GetPlayerController` 0))
  (`WidgetLayoutLibrary.RemoveAllWidgets`)
  (`UserWidget.AddToViewport` (`self.WidgetListEdit`) 0))

(event `/Game/Football/Interface/InterFaceListView.OnClickSave`
  (bind _pawnpositions (`/Game/Football/Factory/FormationFactory.GetPawnPositions` (`self.FormationFactory`)))
  (`/Game/Football/SaveObject/SO_FormationData.SetFormationAt` (`self.FormationData`) (`self.CurrentId`) _pawnpositions))

(event `/Game/Football/Interface/InterFaceListView.OnClickBack`
  ;[1 1 1] Move back one widget
  (`self.DisableInput` self (`GameplayStatics.GetPlayerController` 0))
  (`WidgetLayoutLibrary.RemoveAllWidgets`)
  (`UserWidget.AddToViewport` (`self.WidgetList`) 0))

(fn `SetUpCamera`
  (bind _returnvalue (`|SpawnActorFromClass` "/Script/Engine.CameraActor" (`KismetMathLibrary.MakeTransform` (0.0 0.0 3000.0) (struct :`Pitch` -90.0)) "Undefined" "OverrideRootScale" null null))
  (`PlayerController.SetViewTargetWithBlend` (`GameplayStatics.GetPlayerController` 0) _returnvalue 0.0 "VTBlend_Linear" 0.0 false))

(fn `SetUpFormationData`
  (bind _returnvalue (`GameplayStatics.DoesSaveGameExist` (`self.SaveSlotName`)))
  (if _returnvalue
    (bind _returnvalue_2 (`GameplayStatics.LoadGameFromSlot` (`self.SaveSlotName`)))
    (bind _asso_formation_data (cast `/Game/Football/SaveObject/SO_FormationData` _returnvalue_2))
    (set `self.FormationData` _asso_formation_data)
    (else
      (bind _returnvalue_3 (`GameplayStatics.CreateSaveGameObject` "/Game/Football/SaveObject/SO_FormationData.SO_FormationData_C"))
      (set `self.FormationData` _returnvalue_3))))

(fn `SetUpFormationFactory`
  (bind _returnvalue (`|SpawnActorFromClass` "/Game/Football/Factory/FormationFactory.FormationFactory_C" (`self.ZeroTransform`) "Undefined" "OverrideRootScale" null null))
  (bind _output_get (set `self.FormationFactory` _returnvalue))
  (`/Game/Football/Factory/FormationFactory.SetLevelBlueprint` _output_get self))

(fn `SetUpWidget`
  (`|ExecutionSequence`
    (:`then_0`
      (bind _returnvalue (`|CreateWidget` "/Game/Football/Widget/Wg_List.WG_List_C" (`GameplayStatics.GetPlayerController` 0)))
      (bind _output_get (set `self.WidgetList` _returnvalue))
      (`UserWidget.AddToViewport` _output_get 0)
      (set `/Game/Football/Widget/Wg_List.WidgetType` (`self.WidgetType`) (`self.WidgetList`))
      (set `/Game/Football/Widget/Wg_List.LevelBlueprint` self (`self.WidgetList`))
      (`/Game/Football/Widget/Wg_List.RemoveBtnBack` (`self.WidgetList`))
      (`/Game/Football/SaveObject/SO_Texts.CheckEmpty` (`self.FormationData`) "NewEnumerator2")
      (`/Game/Football/Widget/Wg_List.LoadList` (`self.WidgetList`) (`/Game/Football/SaveObject/SO_Texts.Texts` (`self.FormationData`))))
    (:`then_1`
      ;[1 1 1] Create edit widget
      (bind _returnvalue_2 (`|CreateWidget` "/Game/Football/Widget/WG_ListEdit.WG_ListEdit_C" (`GameplayStatics.GetPlayerController` 0)))
      (bind _output_get_2 (set `self.WidgetListEdit` _returnvalue_2))
      (set `/Game/Football/Widget/WG_ListEdit.LevelBlueprint` self _output_get_2))))

(fn `UserConstructionScript`)